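; BP_LightStand is an actor that continuously moves its Light component back and forth between the Light's starting position and a Target component's position.
; BeginPlay records both relative locations, and Tick accumulates time to drive a sinusoidal in-out ease between them.
; When the elapsed time exceeds EaseTime, the endpoints swap and the timer resets, producing an endless ping-pong motion.
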(event `self.ReceiveBeginPlay`
  (set `self.SourceLocation` (`SceneComponent.RelativeLocation` (`self.Light`)))
  (set `self.TargetLocation` (`SceneComponent.RelativeLocation` (`self.Target`))))

(event `self.ReceiveTick`
  (params (DeltaSeconds :type "Float (single-precision)"))
  (bind _output_get (set `self.CurrentEaseTime` (+ DeltaSeconds (`self.CurrentEaseTime`))))
  (bind _returnvalue (/ _output_get (`self.EaseTime`)))
  (if (> _returnvalue 1.0)
    (bind _output_get_2 (set `self.TempLocation` (`self.TargetLocation`)))
    (set `self.TargetLocation` (`self.SourceLocation`))
    (set `self.SourceLocation` _output_get_2)
    (set `self.CurrentEaseTime` 0.0)
    (else
      (`SceneComponent.K2_SetRelativeLocation` (`self.Light`) (`|EaseFunction` "SinusoidalInOut" _returnvalue (`self.SourceLocation`) (`self.TargetLocation`)) false false))))

(fn `UserConstructionScript`)