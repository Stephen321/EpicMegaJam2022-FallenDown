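; BP_Button is a clickable colour button for the first minigame, reporting presses to a Monitor actor.
; Clicking its Cylinder component compares the ButtonColour string against Blue, Red and Green.
; The matching branch calls BluePressed, RedPressed or GreenPressed on the Monitor reference, and any other value does nothing.
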(event `self.ReceiveBeginPlay`)

(event `self.Cylinder.OnClicked`
  (params (TouchedComponent :type "PrimitiveComponent Object Reference") (ButtonPressed :type "Key Structure"))
  (bind _monitor (`self.Monitor`))
  (bind _button_colour (`self.Button_Colour`))
  (if (`KismetStringLibrary.EqualEqual_StrStr` _button_colour "Blue")
    (`/Game/Core/Gameplay/Minigame_one/BP_Monitor.Blue Pressed` _monitor)
    (elif (`KismetStringLibrary.EqualEqual_StrStr` _button_colour "Red")
      (`/Game/Core/Gameplay/Minigame_one/BP_Monitor.Red Pressed` _monitor)
      (elif (`KismetStringLibrary.EqualEqual_StrStr` _button_colour "Green")
        (`/Game/Core/Gameplay/Minigame_one/BP_Monitor.Green Pressed` _monitor)))))

(fn `UserConstructionScript`)