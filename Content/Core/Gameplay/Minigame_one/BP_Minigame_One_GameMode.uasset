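; Game mode for minigame one, a timed button-press challenge that shifts a Heaven/Hell resource balance.
; The first correct press starts the Tick countdown; later ones push toward Heaven, with streak bonuses, and ResetTime retunes the limit in randomized tiers.
; Incorrect input pushes toward Heaven and timeout toward Hell, both resetting the round.
; Balance thresholds halt play; Maxed records the result, saves and opens the game-over level.
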(event `EndGameByIncorrectInput`
  (`JamResourceSubsystem.ChangeBalance` (subsystem `JamResourceSubsystem`) "Heaven" "Large")
  (set `self.Started` false :!label _label)
  (`self.InitializeVariables`)
  (set `self.Correct Presses` 0)
  (`KismetSystemLibrary.Delay` 1.0)
  (`/Game/Core/Gameplay/Minigame_one/BP_Control_Panel.Activate A Button` (`self.ControlPanel`)))

(event `EndGameByTimeout`
  (bind _returnvalue (`GameplayStatics.GetActorOfClass` "/Game/Core/Gameplay/Minigame_one/BP_Control_Panel.BP_Control_Panel_C"))
  (`/Game/Core/Gameplay/Minigame_one/BP_Control_Panel.DeactivateAllButtons` _returnvalue)
  (`/Game/Core/Gameplay/Minigame_one/BP_Control_Panel.TurnOffMonitor` _returnvalue)
  (`JamResourceSubsystem.ChangeBalance` (subsystem `JamResourceSubsystem`) "Hell" "Medium")
  (goto _label))

(event `Pressed Corectly`
  (if (`self.Started`)
    (bind _result (`/Engine/EditorBlueprintResources/StandardMacros.IncrementInt` (`self.Correct Presses`))
      (:`  `
        (set `self.Correct Presses` _result)
        (`self.ResetTime`)
        (`JamResourceSubsystem.ChangeBalance` (subsystem `JamResourceSubsystem`) "Heaven" "Small")
        (if (> (`self.Correct Presses`) 15)
          (`JamResourceSubsystem.ChangeBalance` (subsystem `JamResourceSubsystem`) "Heaven" "Small")
          (if (> (`self.Correct Presses`) 30)
            (`JamResourceSubsystem.ChangeBalance` (subsystem `JamResourceSubsystem`) "Heaven" "Small")
            (if (> (`self.Correct Presses`) 50)
              (`JamResourceSubsystem.ChangeBalance` (subsystem `JamResourceSubsystem`) "Heaven" "Small"))))))
    (else
      (set `self.Started` true)
      (bind _result_2 (`/Engine/EditorBlueprintResources/StandardMacros.IncrementInt` (`self.Correct Presses`))
        (:`  `
          (set `self.Correct Presses` _result_2))))))

(event `self.ReceiveBeginPlay`
  (bind _returnvalue (`GameplayStatics.GetPlayerController` 0))
  (`self.InitializeVariables`)
  (bind _returnvalue_2 (`|CreateWidget` "/Game/UI/WBP_LevelHUD_MinigameOne.WBP_LevelHUD_MinigameOne_C" _returnvalue))
  (`UserWidget.AddToViewport` _returnvalue_2 0)
  (`WidgetBlueprintLibrary.SetInputMode_GameAndUIEx` _returnvalue _returnvalue_2)
  (add `JamResourceSubsystem.OnBalanceThresholdReached` (subsystem `JamResourceSubsystem`) (delegate `OnBalanceThresholdReached`)))

(event `OnBalanceThresholdReached`
  (params (BalanceType :type "EJamBalanceType Enum" :default "Hell") (Threshold :type "EJamBalanceThreshold Enum" :default "NoChange"))
  (set `self.GameOver` true)
  (`/Game/Core/Gameplay/Minigame_one/BP_Control_Panel.DeactivateAllButtons` (`self.ControlPanel`))
  (`/Game/Core/Gameplay/Minigame_one/BP_Control_Panel.TurnOffMonitor` (`self.ControlPanel`))
  (switch `EJamBalanceThreshold` Threshold
    (:`Maxed`
      ;[1 1 1] TODO: shouldnt have game state here
      (bind _asbp_jam_game_state (cast `/Game/Core/Gameplay/BP_JamGameState` (`GameplayStatics.GetGameState`)))
      (set `JamGameStateBase.bGameWon` (`|EnumEquality` BalanceType "Heaven") _asbp_jam_game_state)
      (`KismetSystemLibrary.Delay` 2.0)
      ;[1 1 1] TODO: figure out how to default to self in ufunction
      (`JamHelperFunctionLibrary.SaveGame` self)
      (`GameplayStatics.OpenLevelBySoftObjectPtr` "/Game/Maps/L_GameOver.L_GameOver"))))

(event `self.ReceiveTick`
  (params (DeltaSeconds :type "Float (single-precision)"))
  (bind _returnvalue (- (`self.SecondsToPress`) DeltaSeconds))
  (if (`self.GameOver`)
    _
    (elif (`self.Started`)
      (if (> _returnvalue 0.0)
        (set `self.SecondsToPress` _returnvalue)
        (else
          (set `self.SecondsToPress` 0.0)
          (`self.EndGameByTimeout`))))))

(fn `InitializeVariables`
  (set `self.Started` false)
  (bind _output_get (set `self.StartingTimeLimit` 15.0))
  (bind _output_get_2 (set `self.SecondsToPress` _output_get))
  (set `self.CurrentTimeLimit` _output_get_2))

(fn `ResetTime`
  (locals (SecondsDivider :type "Float (double-precision)"))
  (bind _returnvalue (* (`self.CurrentTimeLimit`) (`local.SecondsDivider`)))
  (if (> (`self.CurrentTimeLimit`) 10.0)
    (set `local.SecondsDivider` 0.8)
    (set `self.CurrentTimeLimit` (+ (`self.CurrentTimeLimit`) (* (/ (`self.CurrentTimeLimit`) (`local.SecondsDivider`)) 0.02)))
    (if (> _returnvalue 0.6) :!label _label
      (set `self.CurrentTimeLimit` _returnvalue)
      (set `self.SecondsToPress` (`self.CurrentTimeLimit`))
      (else
        (set `self.SecondsToPress` (`self.CurrentTimeLimit`))))
    (elif (> (`self.CurrentTimeLimit`) 7.5)
      (set `local.SecondsDivider` 0.7)
      (set `self.CurrentTimeLimit` (+ (`self.CurrentTimeLimit`) (`KismetMathLibrary.RandomFloatInRange` 0.1 0.6)))
      (goto _label)
      (elif (> (`self.CurrentTimeLimit`) 3.0)
        (bind _output_get (set `local.SecondsDivider` 0.9))
        (set `self.CurrentTimeLimit` (+ (`self.CurrentTimeLimit`) (+ (* (* _output_get (/ (- (`self.CurrentTimeLimit`) 3.0) 4.5)) 0.3) (`KismetMathLibrary.RandomFloatInRange` 0.1 0.4))))
        (goto _label)))))

(fn `UserConstructionScript`)