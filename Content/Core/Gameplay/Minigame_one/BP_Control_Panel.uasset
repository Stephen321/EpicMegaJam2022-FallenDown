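; BP_Control_Panel runs the button-press loop of Minigame One, keeping track of which button is active.
; Its construction script gathers every BP_Button in the level, and BeginPlay activates a random one.
; A correct press notifies the game mode and activates another, rerolling to avoid immediate repeats.
; An incorrect press deactivates all buttons, resets the monitor material, plays every alarm and ends the game through the game mode.
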(event `Button Pressed Incorrectly`
  (bind _asbp_minigame_one_game_mode (cast `/Game/Core/Gameplay/Minigame_one/BP_Minigame_One_GameMode` (`GameplayStatics.GetGameMode`)))
  (`self.DeactivateAllButtons`)
  (`self.TurnOffMonitor`)
  (bind _outactors (`GameplayStatics.GetAllActorsOfClass` "/Game/Core/Gameplay/Minigame_one/BP_Alarm.BP_Alarm_C"))
  (for _array_element _outactors
    (bind _asbp_alarm (cast `/Game/Core/Gameplay/Minigame_one/BP_Alarm` _array_element))
    (`/Game/Core/Gameplay/Minigame_one/BP_Alarm.Play Alarm` _asbp_alarm))
  (`/Game/Core/Gameplay/Minigame_one/BP_Minigame_One_GameMode.EndGameByIncorrectInput` _asbp_minigame_one_game_mode))

(event `Button Pressed Correctly`
  (bind _asbp_minigame_one_game_mode (cast `/Game/Core/Gameplay/Minigame_one/BP_Minigame_One_GameMode` (`GameplayStatics.GetGameMode`)))
  (`/Game/Core/Gameplay/Minigame_one/BP_Minigame_One_GameMode.Pressed Corectly` _asbp_minigame_one_game_mode)
  (`self.Activate A Button`))

(event `self.ReceiveBeginPlay`
  (`self.Activate A Button`))

(fn `Activate A Button`
  (locals (ButtonToSelect :type "/Game/Core/Gameplay/Minigame_one/BP_Button Object Reference"))
  (set `local.ButtonToSelect` (`KismetArrayLibrary.Array_Random` (`self.Buttons`)))
  (while (== (`local.ButtonToSelect`) (`self.LastActivated`))
    (bind _output_get (set `local.ButtonToSelect` (`KismetArrayLibrary.Array_Random` (`self.Buttons`)))))
  (`/Game/Core/Gameplay/Minigame_one/BP_Button.SetActiveButton` _output_get)
  (set `self.LastActivated` _output_get))

(fn `DeactivateAllButtons`
  (for _array_element (`self.Buttons`)
    (`/Game/Core/Gameplay/Minigame_one/BP_Button.SetInactiveButton` _array_element)))

(fn `TurnOffMonitor`
  (`PrimitiveComponent.SetMaterial` (`/Game/Core/Gameplay/Minigame_one/BP_Monitor.Cube` (`self.Monitor`)) 0 "/Game/Materials/Minigame_One/M_Monitor_Default.M_Monitor_Default"))

(fn `UserConstructionScript`
  (bind _outactors (`GameplayStatics.GetAllActorsOfClass` "/Game/Core/Gameplay/Minigame_one/BP_Button.BP_Button_C"))
  (set `self.Buttons` _outactors))