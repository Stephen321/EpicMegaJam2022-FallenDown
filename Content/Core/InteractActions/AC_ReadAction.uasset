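; Widget component that serves as a read interaction, showing configurable info text on a WBP_Info_Game widget.
; BeginPlay writes the text into the widget; Interact stores the interactor, toggles visibility and rebinds the interactable's end-overlap event.
; When the interactor leaves the overlap, a retriggerable delay loops until it is beyond a minimum distance from the owner, then hides the widget.
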(event `self.ReceiveBeginPlay`
  (bind _aswbp_info_game (cast `/Game/Core/InteractActions/WBP_Info_Game` (`self.GetUserWidgetObject`)))
  (bind _output_get (set `self.InfoGameWidget` _aswbp_info_game))
  (`/Engine/EditorBlueprintResources/StandardMacros.IsValid` _output_get
    (:`Is Valid`
      (`TextBlock.SetText` (`/Game/Core/InteractActions/WBP_Info_Game.InfoText` _output_get) (`self.InfoText`))
      (`self.RequestRenderUpdate`))))

(event `ComponentEndOverlap`
  (params (OverlappedComponent :type "PrimitiveComponent Object Reference") (OtherActor :type "Actor Object Reference") (OtherComp :type "PrimitiveComponent Object Reference") (OtherBodyIndex :type Integer))
  (bind _interactor (`self.Interactor`))
  (if (== OtherActor _interactor)
    (`KismetSystemLibrary.RetriggerableDelay` (`self.DisappearTime`) :!label _label)
    (if (> (`Actor.GetDistanceTo` _interactor (`self.GetOwner`)) (`self.MinDissappearDistance`))
      (`self.SetVisibility` false)
      (else
        (goto _label)))))

(event `self.Interact`
  (params (InteractableComponent :type "JamInteractableComponent Object Reference") (Interactor :type "Actor Object Reference"))
  (bind _output_get (set `self.InteractableComponent` InteractableComponent))
  (set `self.Interactor` Interactor)
  (remove `self.OnComponentEndOverlap` _output_get (delegate `ComponentEndOverlap`))
  (add `self.OnComponentEndOverlap` _output_get (delegate `ComponentEndOverlap`))
  (bind _aswbp_info_game (cast `/Game/Core/InteractActions/WBP_Info_Game` (`self.GetUserWidgetObject`)))
  (`/Engine/EditorBlueprintResources/StandardMacros.IsValid` _aswbp_info_game
    (:`Is Valid`
      (if (`self.IsVisible`)
        (`self.SetVisibility` false)
        (`self.RequestRenderUpdate`)
        (else
          (`self.SetVisibility` true))))))